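; Possession spell actor with a mana cost that lets the player take control of an NPC it touches.
; On sphere overlap, an unpossessed tagged NPC is possessed and flagged, and the spell explodes.
; An already-possessed NPC instead makes it backfire, with lightning at the ThirdPersonCharacter, damage and disabled player movement.
; A short timer or destruction clears stored lightning and restores walking, while blocking hits just explode the spell.
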(event OnComponentHit(Sphere)
  (params (HitComponent :type Primitive%20Component%20Object%20Reference) (OtherActor :type Actor%20Object%20Reference) (OtherComp :type Primitive%20Component%20Object%20Reference) (NormalImpulse :type Vector :default "0, 0, 0") (Hit :type Hit%20Result%20Structure%20%28by%20ref%29))
  (bind _returnvalue (Transformation|GetActorLocation))
  ;[1 1 1] Hit Wall
  (Actor|DestroyActor)
  (Audio|PlaySoundatLocation "/Game/StarterContent/Audio/Explosion01.Explosion01" _returnvalue "0, 0, 0" 1.0 1.0 0.0 0 0 0)
  (bind _returnvalue_2 (Effects|SpawnEmitteratLocation "/Game/InfinityBladeEffects/Effects/FX_Cines/cinema03/P_CIN_IB_Explosion.P_CIN_IB_Explosion" _returnvalue (Transformation|GetActorRotation)))
  (Utilities|FlowControl|Delay 0.5)
  (Components|DestroyComponent _returnvalue_2))

(event OnComponentBeginOverlap(Sphere)
  (params (OverlappedComponent :type Primitive%20Component%20Object%20Reference) (OtherActor :type Actor%20Object%20Reference) (OtherComp :type Primitive%20Component%20Object%20Reference) (OtherBodyIndex :type Integer) (bFromSweep :type Boolean) (SweepResult :type Hit%20Result%20Structure%20%28by%20ref%29))
  ;[1 1 1] PossesAi
  (CallFunction|PossesNPC OtherActor)
  (Utilities|Time|SetTimerbyFunctionName 0 "Delite Litnings" 0.2))

(event EventBeginPlay)

(event Collision|EventActorBeginOverlap
  (params (OtherActor :type Actor%20Object%20Reference)))

(event EventTick
  (params (DeltaSeconds :type Float%20%28single-precision%29)))

(event EventDestroyed
  (CallFunction|DeliteLitnings))

(fn ConstructionScript
  (Variables|Default|SetManaCost 4e+01))

(fn PossesNPC
  (params (NPC :type Actor%20Object%20Reference))
  (bind _returnvalue (Game|GetPlayerCharacter 0))
  (bind _returnvalue_2 (Transformation|GetActorLocation))
  (if (Actor|ActorHasTag NPC "NPC")
    (bind _asnpc (Utilities|Casting|CastToNPC NPC))
    (if (Variables|/Script/MagicTech.NPC|GetBeenPossed _asnpc)
      (bind _outactors (Actor|GetAllActorsOfClass "/Game/ThirdPersonCPP/Blueprints/ThirdPersonCharacter.ThirdPersonCharacter_C"))
      (bind _returnvalue_3 (Effects|SpawnEmitteratLocation "/Game/InfinityBladeEffects/Effects/FX_Monsters/FX_Monster_Genno/P_Genno_Weapon_Lightning_01.P_Genno_Weapon_Lightning_01" (Transformation|GetActorLocation (Utilities|Array|Get(acopy) _outactors))))
      (Utilities|Array|Add (Variables|Default|GetLinings) _returnvalue_3)
      (Pawn|Components|CharacterMovement|DisableMovement (Variables|/Script/Engine.Character|GetCharacterMovement _returnvalue))
      (Game|Damage|ApplyDamage _returnvalue 1e+01 0 0)
      (else
        (Utilities|FlowControl|Sequence
          (:then_0
            (Actor|DestroyActor)
            (Audio|PlaySoundatLocation "/Game/StarterContent/Audio/Explosion01.Explosion01" _returnvalue_2 "0, 0, 0" 1.0 1.0 0.0 0 0 0)
            (Effects|SpawnEmitteratLocation "/Game/InfinityBladeEffects/Effects/FX_Cines/cinema03/P_CIN_IB_Explosion.P_CIN_IB_Explosion" _returnvalue_2 (Transformation|GetActorRotation)))
          (:then_1
            (Pawn|Possess (Game|GetPlayerController 0) _asnpc)
            (Variables|/Script/MagicTech.NPC|SetBeenPossed _asnpc true)))))))

(fn DeliteLitnings
  (for _array_element (Variables|Default|GetLinings)
    (Utilities|IsValid _array_element
      (:Is%20Valid
        (Components|DestroyComponent _array_element)
        (Pawn|Components|CharacterMovement|SetMovementMode (Variables|/Script/Engine.Character|GetCharacterMovement (Game|GetPlayerCharacter 0)) "MOVE_Walking" 0)))))